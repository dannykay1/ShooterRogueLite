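; BP_Bomber is a Blueprint that shows floating damage text when its SAttribute reports an attribute change.
; The change handler spawns a BP_DamageText at the actor's location, passing the delta as text and a randomized final location offset to either side along world Y and upward.
; It also prints a placeholder string and draws a debug sphere at that final location.
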(event `self.SAttribute.OnAttributeChanged`
  (params (Attribute :type "Attribute Structure") (Delta :type "Float (single-precision)"))
  (bind _returnvalue (`KismetMathLibrary.RandomFloatInRange` 25.0 100.0))
  (`KismetSystemLibrary.PrintString` "Hello")
  (bind _returnvalue_2 (`|SpawnActorFromClass` "/Game/Blueprints/BP_DamageText.BP_DamageText_C" (`KismetMathLibrary.MakeTransform` (`self.K2_GetActorLocation`)) "Undefined" "OverrideRootScale" null (`KismetTextLibrary.Conv_DoubleToText` Delta "HalfToEven") (+ (`self.K2_GetActorLocation`) (`KismetMathLibrary.MakeVector` 0.0 (`KismetMathLibrary.SelectFloat` (* _returnvalue -1.0) _returnvalue (`KismetMathLibrary.RandomBool`)) (`KismetMathLibrary.RandomFloatInRange` 30.0 100.0))) null))
  (`KismetSystemLibrary.DrawDebugSphere` (`/Game/Blueprints/BP_DamageText.FinalLocation` _returnvalue_2) 10.0 12 (struct :`R` 1.0 :`G` 1.0 :`A` 1.0) 3.0 1.0))

(fn `UserConstructionScript`)