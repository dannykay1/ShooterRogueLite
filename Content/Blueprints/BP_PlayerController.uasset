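; BP_PlayerController is a player controller Blueprint that prints debug readouts of the player's inventory on possession.
; On possess, it prints each InventoryData key as an inventory entry, then the name of each valid SlottedItems value, as long-lived screen messages.
; A disconnected chain that would call NotifyInventoryLoaded after a delay and print a confirmation never runs.
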(event `self.ReceivePossess`
  (params (PossessedPawn :type "Pawn Object Reference"))
  (bind _keys (`BlueprintMapLibrary.Map_Keys` (`self.InventoryData`)))
  (for _array_element _keys
    (`KismetSystemLibrary.PrintString` (`KismetTextLibrary.Conv_TextToString` (`|FormatText` "Inventory {item}" _array_element)) true true (struct :`G` 0.66 :`B` 1.0 :`A` 1.0) 20.0))
  (bind _values (`BlueprintMapLibrary.Map_Values` (`self.SlottedItems`)))
  (for _array_element_2 _values
    (`/Engine/EditorBlueprintResources/StandardMacros.IsValid` _array_element_2
      (:`Is Valid`
        (`KismetSystemLibrary.PrintString` (`KismetTextLibrary.Conv_TextToString` (`|FormatText` "Slotted {item}" (`SItem.ItemName` _array_element_2))) true true (struct :`G` 0.66 :`B` 1.0 :`A` 1.0) 20.0)))))

(fn `UserConstructionScript`)