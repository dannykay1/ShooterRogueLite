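; Player character Blueprint that sets up the HUD and a randomly tinted gun stock on BeginPlay.
; Aim, fire and sprint inputs start and stop gameplay-tagged actions on ActionComponent, with successful aim changes driving a timeline that blends camera FOV.
; Keys 1 and 2 apply test damage to Health and Armor, and AttributeComponent changes only print a debug string.
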(event `self.ReceiveBeginPlay`
  (bind _weaponmesh (`self.WeaponMesh`))
  (`|ExecutionSequence`
    (:`then_0`
      (bind _returnvalue (`PrimitiveComponent.CreateDynamicMaterialInstance` _weaponmesh 0 (`PrimitiveComponent.GetMaterial` _weaponmesh 0) "None"))
      (`MaterialInstanceDynamic.SetVectorParameterValue` _returnvalue "ColorGunStock" (select `int` (`KismetMathLibrary.RandomInteger` 4) :`0` (struct :`R` 1.0 :`G` 1.0 :`B` 1.0 :`A` 1.0) :`1` (struct :`G` 1.0 :`A` 1.0) :`2` (struct :`G` 0.695381 :`B` 1.0 :`A` 1.0) :`3` (struct :`R` 1.0 :`G` 1.0 :`A` 1.0) :!type "LinearColor Structure")))
    (:`then_1`
      (bind _returnvalue_2 (`|CreateWidget` "/Game/UI/Widgets/WBP_HUD.WBP_HUD_C" (`GameplayStatics.GetPlayerController` 0)))
      (`UserWidget.AddToViewport` _returnvalue_2 0))))

(event `InputAction|AimDownSights`
  (params (Key :type "Key Structure"))
  (bind _actioncomponent (`self.ActionComponent`))
  (:`Pressed`
    (bind _returnvalue (`SActionComponent.StartAction` _actioncomponent self (struct :`TagName` "Action.AimDownSights")))
    (if _returnvalue
      (bind (_direction _aimdelta) (`Timeline|AimDownSights` :!label _label)
        (:`Update`
          (bind _output_get (set `self.Aim Delta` _aimdelta))
          (`CameraComponent.SetFieldOfView` (`self.CameraComponent`) (`KismetMathLibrary.Lerp` 90.0 65.0 _output_get))))))
  (:`Released`
    (bind _returnvalue_2 (`SActionComponent.StopAction` _actioncomponent self (struct :`TagName` "Action.AimDownSights")))
    (if _returnvalue_2
      (goto _label :!via `Reverse`))))

(event `InputAction|PrimaryFire`
  (params (Key :type "Key Structure"))
  (bind _actioncomponent (`self.ActionComponent`))
  (:`Pressed`
    (`SActionComponent.StartAction` _actioncomponent self (struct :`TagName` "Action.Shoot")))
  (:`Released`
    (`SActionComponent.StopAction` _actioncomponent self (struct :`TagName` "Action.Shoot"))))

(event `InputAction|Sprint`
  (params (Key :type "Key Structure"))
  (bind _actioncomponent (`self.ActionComponent`))
  (:`Pressed`
    (`SActionComponent.StartAction` _actioncomponent self (struct :`TagName` "Action.Sprint")))
  (:`Released`
    (`SActionComponent.StopAction` _actioncomponent self (struct :`TagName` "Action.Sprint"))))

(event `Key|One`
  (params (Key :type "Key Structure"))
  (:`Pressed`
    (`SBlueprintLibrary.ApplyDamage` self (struct :`TagName` "Attribute.Health") 10.0)))

(event `Key|Two`
  (params (Key :type "Key Structure"))
  (:`Pressed`
    (`SBlueprintLibrary.ApplyDamage` self (struct :`TagName` "Attribute.Armor") 10.0)))

(event `self.AttributeComponent.OnAttributeChanged`
  (params (Attribute :type "Attribute Structure"))
  (`KismetSystemLibrary.PrintString` "Hello"))

(fn `UserConstructionScript`)