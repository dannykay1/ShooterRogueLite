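; Floating damage text actor that shows a text and color through a widget component and drifts to a randomized spot.
; On BeginPlay it picks a target with random sideways and upward offsets, passes Text and Color to WBP_DamageText, and sets a lifespan for self-removal.
; Tick eases the actor toward that target with VInterpTo.
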(event `self.ReceiveBeginPlay`
  (`|ExecutionSequence`
    (:`then_0`
      (bind _output_get (set `self.StartLocation` (`self.K2_GetActorLocation`)))
      (set `self.FinalLocation` (+ _output_get (`KismetMathLibrary.MakeVector` 0.0 (`KismetMathLibrary.RandomFloatInRange` -50.0 50.0) (`KismetMathLibrary.RandomFloatInRange` 0.0 300.0)))))
    (:`then_1`
      (bind _aswbp_damage_text (cast `/Game/UI/Widgets/WBP_DamageText` (`WidgetComponent.GetUserWidgetObject` (`self.Widget`))))
      (set `/Game/UI/Widgets/WBP_DamageText.Text` (`self.Text`) _aswbp_damage_text)
      (set `/Game/UI/Widgets/WBP_DamageText.Color` (`self.Color`) _aswbp_damage_text))
    (:`then_2`
      (`self.SetLifeSpan` 10.0))))

(event `self.ReceiveTick`
  (params (DeltaSeconds :type "Float (single-precision)"))
  (bind _output_get (set `self.StartLocation` (`KismetMathLibrary.VInterpTo` (`self.StartLocation`) (`self.FinalLocation`) DeltaSeconds 3.0)))
  (`self.K2_SetActorLocation` _output_get))

(fn `UserConstructionScript`)