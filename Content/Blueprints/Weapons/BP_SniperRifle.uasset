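; BP_SniperRifle is a sniper rifle with a randomly colored stock and an adjustable scene-capture zoom.
; On BeginPlay it creates a dynamic material on the mesh's first slot and sets the gun stock color to one of four presets at random.
; The SetFieldOfFiew event adds a delta to the SceneCaptureComponent2D FOV, clamps it to a fixed range and prints the result on screen.
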(event `self.ReceiveBeginPlay`
  (bind _meshcomp (`self.MeshComp`))
  (bind _returnvalue (`PrimitiveComponent.CreateDynamicMaterialInstance` _meshcomp 0 (`PrimitiveComponent.GetMaterial` _meshcomp 0) "None"))
  (`MaterialInstanceDynamic.SetVectorParameterValue` _returnvalue "ColorGunStock" (select `int` (`KismetMathLibrary.RandomInteger` 4) :`0` (struct :`R` 1.0 :`G` 1.0 :`B` 1.0 :`A` 1.0) :`1` (struct :`G` 1.0 :`A` 1.0) :`2` (struct :`G` 0.695381 :`B` 1.0 :`A` 1.0) :`3` (struct :`R` 1.0 :`G` 1.0 :`A` 1.0) :!type "LinearColor Structure")))

(event `SetFieldOfFiew`
  (params (Delta :type "Float (double-precision)"))
  (bind _output_get (set `SceneCaptureComponent2D.FOVAngle` (`KismetMathLibrary.FClamp` (+ Delta (`SceneCaptureComponent2D.FOVAngle` (`self.SceneCaptureComponent2D`))) 5.0 100.0) (`self.SceneCaptureComponent2D`)))
  (`KismetSystemLibrary.PrintString` (`KismetTextLibrary.Conv_TextToString` (`|FormatText` "Weapon FOV: {fov}" _output_get))))

(fn `UserConstructionScript`)