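; BP_AttributeTester is a debug Blueprint that prints the attributes held by its AttributeComp.
; On BeginPlay it iterates the keys of the component's gameplay-tag-keyed Attributes map and looks up each entry.
; Each attribute prints on screen in green with the owner, tag, and current and maximum values, with a fallback message for failed lookups.
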(event `self.ReceiveBeginPlay`
  (bind _attributes (`SAttributeComponent.Attributes` (`self.AttributeComp`)))
  (bind _keys (`BlueprintMapLibrary.Map_Keys` _attributes))
  (for _array_element _keys
    (bind (_value _returnvalue) (`BlueprintMapLibrary.Map_Find` _attributes _array_element))
    (if _returnvalue
      (bind (_tag _currentvalue _maximumvalue) (break `Attribute` _value))
      (`KismetSystemLibrary.PrintString` (`KismetTextLibrary.Conv_TextToString` (`|FormatText` "{MyName} {Tag} {0} / {1}" self (`BlueprintGameplayTagLibrary.GetDebugStringFromGameplayTag` _array_element) _currentvalue _maximumvalue)) true true (struct :`G` 1.0 :`A` 1.0) 5.0)
      (else
        (`KismetSystemLibrary.PrintString` "Didnt find attribute")))))

(event `self.ReceiveTick`
  (params (DeltaSeconds :type "Float (single-precision)")))

(fn `UserConstructionScript`)