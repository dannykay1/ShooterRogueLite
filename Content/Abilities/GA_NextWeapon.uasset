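; GA_NextWeapon is a gameplay ability that switches the player's weapon to the pistol.
; On activation it commits, then plays the FPP rifle equip montage on the owning skeletal mesh.
; As the montage starts, it sets BP_Player's weapon mesh to a hardcoded Darkness_Pistol and tells AnimBP_Player to refresh via UpdateInfo.
; The ability ends when the montage completes, blends out or is interrupted.
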(event `self.K2_ActivateAbility`
  (bind _returnvalue (`self.GetOwningComponentFromActorInfo`))
  (`self.K2_CommitAbility`)
  (`|PlayMontage` _returnvalue "/Game/FirstPersonCharacter/Animations/FPP_RifleEquip_Montage.FPP_RifleEquip_Montage"
    (:`then`
      (`SkinnedMeshComponent.SetSkinnedAssetAndUpdate` (`/Game/Blueprints/BP_Player.WeaponMesh` (cast `/Game/Blueprints/BP_Player` (`self.GetAvatarActorFromActorInfo`) :!pure true)) "/Game/SciFiWeapDark/Weapons/Darkness_Pistol.Darkness_Pistol" true)
      (`/Game/FirstPersonCharacter/Animations/AnimBP_Player.UpdateInfo` (cast `/Game/FirstPersonCharacter/Animations/AnimBP_Player` (`SkeletalMeshComponent.GetAnimInstance` _returnvalue) :!pure true)))
    (:`OnCompleted`
      (`self.K2_EndAbility` :!label _label))
    (:`OnBlendOut`
      (goto _label))
    (:`OnInterrupted`
      (goto _label))))